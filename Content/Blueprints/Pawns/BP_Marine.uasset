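; Player marine pawn for a twin-stick style shooter, with world-axis movement, a HUD, clamped health, a kill counter and a delayed reload of the Mars level on death.
; Every tick it sets yaw from thumbstick direction or smoothed mouse velocity, using deadzones and whichever device last pressed a key.
; Holding fire loops a timer-driven line trace from the rifle muzzle along control rotation, applying damage with impact, flash and sound effects.
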(event EventTick
  (params (DeltaSeconds :type Float%20%28single-precision%29))
  (WeaponFunctions|UpdatePlayerAim))

(event EventBeginPlay
  (bind _returnvalue (UserInterface|CreateWidget "/Game/UI/W_PlayerHUD.W_PlayerHUD_C" 0 self))
  (UserInterface|Viewport|AddtoViewport _returnvalue 0))

(event Game|Damage|EventAnyDamage
  (params (Damage :type Float%20%28single-precision%29) (DamageType :type Damage%20Type%20Object%20Reference) (InstigatedBy :type Controller%20Object%20Reference) (DamageCauser :type Actor%20Object%20Reference))
  (if (PlayerFunctions|IsAlive)
    (bind _hp (PlayerFunctions|DecreaseHP Damage))
    (if (== _hp 0.0)
      (Variables|PlayerProperties|SetIsDead true)
      (WeaponFunctions|StopFiringWeapon)
      (Utilities|FlowControl|Delay 4.0)
      (Game|OpenLevel(byName) "Mars"))))

(event Input|ActionEvents|InputActionFireWeapon
  (params (Key :type Key%20Structure :default "None"))
  (:Pressed
    (WeaponFunctions|StartFiringWeapon))
  (:Released
    (WeaponFunctions|StopFiringWeapon)))

(event Input|AxisEvents|InputAxisMoveUp
  (params (AxisValue :type Float%20%28single-precision%29))
  (if (PlayerFunctions|IsAlive)
    (Pawn|Input|AddMovementInput "1.000000, 0, 0" AxisValue false)))

(event Input|AxisEvents|InputAxisMoveRight
  (params (AxisValue :type Float%20%28single-precision%29))
  (if (PlayerFunctions|IsAlive)
    (Pawn|Input|AddMovementInput "0.000000,1.000000, 0" AxisValue false)))

(event Input|KeyboardEvents|AnyKey
  (params (Key :type Key%20Structure :default "None"))
  (:Pressed
    (Variables|ThumbstickInput|SetGamepadActive (Class|KismetInputLibrary|KeyIsGamepadKey Key))))

(fn ConstructionScript)

(fn UpdatePlayerAim
  (if (PlayerFunctions|IsAlive)
    (if (Variables|ThumbstickInput|GetGamepadActive)
      (ThumbstickInput|UpdateThumbstickAim)
      (else
        (MouseInput|UpdateMouseAim)))))

(fn IsThumbstickAboveDeadzone
  (return (> (Math|Vector2D|Vector2DLength (Math|Vector2D|MakeVector2D (Input|AxisValues|GetThumbstickAimUp) (Input|AxisValues|GetThumbstickAimRight))) (Variables|ThumbstickInput|GetThumbstickDeadzone))))

(fn GetMouseVelocity
  (bind _returnvalue (Game|GetPlayerController 0))
  (bind (_deltax _deltay) (Class|PlayerController|GetInputMouseDelta _returnvalue))
  (return (/ (Math|Vector2D|MakeVector2D _deltax _deltay) (Utilities|Time|GetWorldDeltaSeconds))))

(fn IsMouseAboveDeadzone
  (return (> (Math|Vector2D|Vector2DLength (MouseInput|GetMouseVelocity)) (Variables|MouseInput|GetMouseDeadzone))))

(fn UpdateMouseAim
  (if (MouseInput|IsMouseAboveDeadzone)
    (Pawn|SetControlRotation (Game|GetPlayerController 0) (MouseInput|GetMouseAimDirection))))

(fn GetMouseAimDirection
  (bind _returnvalue (MouseInput|GetMouseVelocity))
  (return (Math|Interpolation|RInterpTo (Pawn|GetControlRotation (Game|GetPlayerController 0) :!class /Script/Engine.Controller) (Math|Rotator|MakeRotator 0.0 0.0 (Class|KismetMathLibrary|DegAtan2 (.x _returnvalue) (.y _returnvalue))) (Utilities|Time|GetWorldDeltaSeconds) (Variables|MouseInput|GetMouseSmoothingStrength))))

(fn UpdateThumbstickAim
  (if (ThumbstickInput|IsThumbstickAboveDeadzone)
    (Pawn|SetControlRotation (Game|GetPlayerController 0) (ThumbstickInput|GetThumbstickAimDirection))))

(fn GetThumbstickAimDirection
  (return (Math|Rotator|MakeRotator 0.0 0.0 (Class|KismetMathLibrary|DegAtan2 (Input|AxisValues|GetThumbstickAimRight) (Input|AxisValues|GetThumbstickAimUp)))))

(fn StartFiringWeapon
  (if (PlayerFunctions|IsAlive)
    (Components|Activation|Activate (Variables|Default|GetP_MuzzleFlash) false)
    (bind _returnvalue (Audio|SpawnSound2D "/Game/Sounds/Weapon_AssaultRifle/Stereo/RifleFireLoop_Cue.RifleFireLoop_Cue" 1.0 1.0 0.0 0))
    (Variables|Default|SetWeaponFireSound _returnvalue)
    (WeaponFunctions|WeaponTrace)
    (Utilities|Time|SetTimerbyFunctionName 0 "WeaponTrace" (Variables|WeaponProperties|GetWeaponFireRate) true)))

(fn StopFiringWeapon
  (bind _weaponfiresound (Variables|Default|GetWeaponFireSound))
  (Components|Activation|Deactivate (Variables|Default|GetP_MuzzleFlash))
  (Utilities|IsValid _weaponfiresound
    (:Is%20Valid
      (Audio|Components|Audio|Stop _weaponfiresound)
      (Utilities|Time|ClearTimerbyFunctionName 0 "WeaponTrace")
      (if (PlayerFunctions|IsAlive)
        (Audio|PlaySound2D "/Game/Sounds/Weapon_AssaultRifle/Stereo/RifleFireEnd_Cue.RifleFireEnd_Cue" 1.0 1.0 0.0 0 0)))))

(fn DecreaseHP
  (params (DamageAmount :type Float%20%28single-precision%29))
  (bind _output_get (Variables|PlayerProperties|SetPlayerHP (Math|Float|Clamp(Float) (- (Variables|PlayerProperties|GetPlayerHP) DamageAmount) 0.0 1e+02)))
  (return _output_get))

(fn IsAlive
  (return (not (Variables|PlayerProperties|GetIsDead))))

(fn WeaponTrace
  (bind _outhit (Collision|LineTraceByChannel (WeaponFunctions|GetWeaponTraceStartLocation) (WeaponFunctions|GerWeaponTraceEndLocation) "TraceTypeQuery1" false 0 "None"))
  (if (.bBlockingHit (Collision|BreakHitResult _outhit))
    (WeaponFunctions|SpawnImpactHit (.ImpactPoint (Collision|BreakHitResult _outhit)))
    (Game|Damage|ApplyDamage (.HitActor (Collision|BreakHitResult _outhit)) (Variables|WeaponProperties|GetDamagePerShot) 0 0)))

(fn GetWeaponTraceStartLocation
  (return (Transformation|GetSocketLocation (Variables|Default|GetRifle) "MuzzleFlash")))

(fn GerWeaponTraceEndLocation
  (return (+ (WeaponFunctions|GetWeaponTraceStartLocation) (* (Math|Vector|GetForwardVector (Pawn|GetControlRotation :!class /Script/Engine.Pawn)) (Variables|WeaponProperties|GetWeaponRange)))))

(fn IncreaseKills
  (Math|Integer|IncrementInt (Variables|PlayerProperties|GetPlayerKills)))

(fn SpawnImpactHit
  (params (HitLocation :type Vector))
  (Effects|SpawnEmitteratLocation "/Game/Effects/Weapons/Impacts/P_AssaultRifle_IH.P_AssaultRifle_IH" HitLocation))

(fn AddHealth
  (params (HealthToAdd :type Float%20%28single-precision%29))
  (Variables|PlayerProperties|SetPlayerHP (Math|Float|Clamp(Float) (+ (Variables|PlayerProperties|GetPlayerHP) HealthToAdd) 0.0 1e+02)))

(fn IsHealthFull
  (return (== (Variables|PlayerProperties|GetPlayerHP) 1e+02)))